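; Phantom variant of an interactive level platform that ties its timeline-driven movement to Show and Hide events.
; On BeginPlay it runs the parent logic, then calls Hide only if the first overlapping SideScrollerCharacter casts successfully.
; When ShouldMove is set, Show starts the timeline and Hide stops it.
; Tick and overlap events are disabled, and construction just defers to the parent.
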(event EventBeginPlay
  (|CallParentFunction)
  (Utilities|Casting|CastToSideScrollerCharacter (Utilities|Array|Get(acopy) (Collision|GetOverlappingActors "/Game/Blueprint/Blueprints/SideScrollerCharacter.SideScrollerCharacter_C" :!class /Script/Engine.Actor)))
  (CallFunction|Hide))

(event Collision|EventActorBeginOverlap
  (params (OtherActor :type Actor%20Object%20Reference))
  (|CallParentFunction OtherActor) ; This node is disabled and will not be called.\nDrag off pins to build functionality.
)

(event EventTick
  (params (DeltaSeconds :type Float%20%28single-precision%29)))

(event EventHide
  (if (Variables|Default|GetshouldMove)
    (CallFunction|StopTimeline)))

(event EventShow
  (if (Variables|Default|GetshouldMove)
    (CallFunction|StartTimeline)))

(fn ConstructionScript
  (|CallParentFunction))