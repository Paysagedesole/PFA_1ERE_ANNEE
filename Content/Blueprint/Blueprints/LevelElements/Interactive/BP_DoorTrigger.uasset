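; BP_DoorTrigger is an interactive level trigger that opens a linked Door once.
; Overlapping its Box registers the trigger as the SideScrollerCharacter's DoorTrigger; the overlap itself does not open anything.
; When OpenDoor is called, it proceeds only if the game mode's NextWorld differs from the trigger's Type and it is unused.
; It then marks itself used, opens the Door if valid and becomes that Door's owner.
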(event OnComponentBeginOverlap(Box)
  (params (OverlappedComponent :type Primitive%20Component%20Object%20Reference) (OtherActor :type Actor%20Object%20Reference) (OtherComp :type Primitive%20Component%20Object%20Reference) (OtherBodyIndex :type Integer) (bFromSweep :type Boolean) (SweepResult :type Hit%20Result%20Structure%20%28by%20ref%29))
  (bind _asside_scroller_character (Utilities|Casting|CastToSideScrollerCharacter OtherActor))
  (Variables|/Game/Blueprint/Blueprints/SideScrollerCharacter.SideScrollerCharacter_C|SetDoorTrigger _asside_scroller_character self))

(event Custom|OpenDoor
  (bind _door (Variables|Default|GetDoor))
  (bind _asbp_gamemode_base (Utilities|Casting|CastToBP_Gamemode_Base (Game|GetGameMode)))
  (if (not (== (Variables|/Game/Blueprint/GameMode/BP_Gamemode_Base.BP_Gamemode_Base_C|GetNextWorld _asbp_gamemode_base) (Variables|Default|GetType)))
    (if (not (Variables|Default|GetisUsed))
      (Variables|Default|SetisUsed true)
      (if (Utilities|IsValid _door)
        (Default|OpenDoor _door)
        (Actor|SetOwner (Variables|Default|GetDoor) self)))))

(event EventBeginPlay
  (|CallParentFunction) ; This node is disabled and will not be called.\nDrag off pins to build functionality.
)

(event Collision|EventActorBeginOverlap
  (params (OtherActor :type Actor%20Object%20Reference)))

(event EventTick
  (params (DeltaSeconds :type Float%20%28single-precision%29)))

(fn ConstructionScript
  (|CallParentFunction))