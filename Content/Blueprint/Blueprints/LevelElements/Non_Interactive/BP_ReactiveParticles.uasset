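; Niagara particle actor that wanders through the side-scroller level in the YZ plane and flees from the player character.
; A self-repeating Move event picks a random direction in a forward cone, line-traces it, then either moves there or turns to the hit normal.
; Repulse overlaps turn it away from the character and temporarily boost movement speed and Niagara attraction and acceleration.
; In menu mode it skips wandering, and Move offsets it vertically by index.
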(event OnComponentBeginOverlap(Repulse)
  (params (OverlappedComponent :type Primitive%20Component%20Object%20Reference) (OtherActor :type Actor%20Object%20Reference) (OtherComp :type Primitive%20Component%20Object%20Reference) (OtherBodyIndex :type Integer) (bFromSweep :type Boolean) (SweepResult :type Hit%20Result%20Structure%20%28by%20ref%29))
  (bind _asside_scroller_character (Utilities|Casting|CastToSideScrollerCharacter OtherActor))
  (Transformation|SetWorldRotation (Variables|Default|GetDefaultSceneRoot) (Math|Conversions|RotationFromXVector (- (Transformation|GetWorldLocation (Variables|Default|GetDefaultSceneRoot)) (Transformation|GetActorLocation _asside_scroller_character))) false false)
  (CallFunction|ChangeParameters true)
  (CallFunction|Move))

(event Custom|Move
  (params (Index :type Integer))
  (bind _defaultsceneroot (Variables|Default|GetDefaultSceneRoot))
  (bind _returnvalue (Transformation|GetWorldLocation _defaultsceneroot))
  (Development|PrintString (Utilities|String|ToString(Integer) Index) true true "(R=1.000000,G=0.381227,B=0.000000,A=1.000000)")
  (if (Math|Boolean|Equal(Boolean) (Variables|Default|GetisMenu) false)
    (bind _output_get (Variables|Default|SetRandom (Math|Vector|Normalize (Math|Random|RandomUnitVectorinConeinDegrees (Math|Vector|GetForwardVector (Transformation|GetWorldRotation (Variables|Default|GetDefaultSceneRoot))) 15.0))))
    (bind (_outhit _returnvalue_2) (Collision|LineTraceForObjects _returnvalue (+ _returnvalue (Math|Vector|MakeVector 0.0 (.y (* _output_get 1.1e+02)) (.z (* _output_get 1.1e+02)))) (Utilities|Array|MakeArray "ObjectTypeQuery1" "ObjectTypeQuery2") false (Utilities|Array|MakeArray (Variables|Default|GetCharacterRef)) "None"))
    (if _returnvalue_2
      (Transformation|SetWorldRotation (Variables|Default|GetDefaultSceneRoot) (Math|Rotator|MakeRotator (.roll (Math|Conversions|RotationFromXVector (Math|Vector|MakeVector (.x (.ImpactNormal (Collision|BreakHitResult _outhit))) (.y (.ImpactNormal (Collision|BreakHitResult _outhit))) (.z (.ImpactNormal (Collision|BreakHitResult _outhit)))))) (.pitch (Math|Conversions|RotationFromXVector (Math|Vector|MakeVector (.x (.ImpactNormal (Collision|BreakHitResult _outhit))) (.y (.ImpactNormal (Collision|BreakHitResult _outhit))) (.z (.ImpactNormal (Collision|BreakHitResult _outhit)))))) (.yaw (Math|Conversions|RotationFromXVector (Math|Vector|MakeVector (.x (.ImpactNormal (Collision|BreakHitResult _outhit))) (.y (.ImpactNormal (Collision|BreakHitResult _outhit))) (.z (.ImpactNormal (Collision|BreakHitResult _outhit))))))) false false)
      (Utilities|FlowControl|Delay 0.2)
      (CallFunction|Move)
      (else
        (Components|MoveComponentTo (Variables|Default|GetDefaultSceneRoot) (+ _returnvalue (Math|Vector|MakeVector 0.0 (.y (* _output_get 1.1e+02)) (.z (* _output_get 1.1e+02)))) (Transformation|GetActorRotation) false false (Variables|Default|GetSpeed) false)
        (CallFunction|ChangeParameters false)
        (Utilities|FlowControl|Delay 0.2)
        (CallFunction|Move)))
    (else
      (Transformation|SetWorldLocation (Variables|Default|GetDefaultSceneRoot) (+ (Transformation|GetWorldLocation (Variables|Default|GetDefaultSceneRoot)) (* "0, 0,150.000000" Index)) false false))))

(event Custom|ChangeParameters
  (params (isFast :type Boolean))
  (bind _niagara (Variables|Default|GetNiagara))
  (bind _niagara_2 (Variables|Default|GetNiagara))
  (bind _attraction (Variables|Default|GetAttraction))
  (bind _acceleration (Variables|Default|GetAcceleration))
  (if isFast
    (Effects|Components|ParticleSystem|SetFloatParameter _niagara_2 "Attraction" (* 2.0 _attraction))
    (Effects|Components|ParticleSystem|SetFloatParameter _niagara_2 "Acceleration" (* 2.0 _acceleration))
    (Variables|Default|SetSpeed 5.0)
    (else
      (Effects|Components|ParticleSystem|SetFloatParameter _niagara "Attraction" _attraction)
      (Effects|Components|ParticleSystem|SetFloatParameter _niagara "Acceleration" _acceleration)
      (Variables|Default|SetSpeed 1e+01))))

(event EventBeginPlay
  (if (not (Variables|Default|GetisMenu))
    (CallFunction|Move)))

(event Collision|EventActorBeginOverlap
  (params (OtherActor :type Actor%20Object%20Reference)))

(event EventTick
  (params (DeltaSeconds :type Float%20%28single-precision%29))
  (Utilities|IsValid (Variables|Default|GetCharacterRef)
    (:Is%20Not%20Valid
      (bind _asside_scroller_character (Utilities|Casting|CastToSideScrollerCharacter (Game|Player|GetPlayerPawn 0)))
      (Variables|Default|SetCharacterRef _asside_scroller_character))))

(fn ConstructionScript
  (bind _niagara (Variables|Default|GetNiagara))
  (Effects|Components|ParticleSystem|SetFloatParameter _niagara "Acceleration" (Variables|Default|GetAcceleration))
  (Effects|Components|ParticleSystem|SetFloatParameter _niagara "Attraction" (Variables|Default|GetAttraction))
  (Transformation|SetActorRotation (Math|Rotator|MakeRotator 0.0 (Variables|Default|GetRotation) 9e+01)))