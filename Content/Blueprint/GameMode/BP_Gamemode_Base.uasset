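; Base game mode for the side-scroller's light/dark world switching, with game over returning to the hub level.
; BeginPlay sorts level elements by type, and ChangeElementType toggles NextWorld (ignoring NewElement), crossfading MPC_Worlds opacities and updating both element sets.
; Entering dark shades the character to black, then starts a timer that kills them.
; Returning to light stops the shading and pauses that timer; Tick caches the character reference.
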(event Custom|ChangeElementType
  (params (New%20Element :type Enum_LevelElementsTypes%20Enum :default "NewEnumerator1") (Is%20Instant :type Boolean))
  (bind _characterref (Variables|Default|GetCharacterRef))
  (bind _lightelements (Variables|Default|GetLightElements))
  (bind _darkelements (Variables|Default|GetDarkElements))
  (Utilities|IsValid _characterref
    (:Is%20Valid
      (Variables|/Game/Blueprint/Blueprints/SideScrollerCharacter.SideScrollerCharacter_C|SetcanChangeWorld _characterref false)
      (switch Utilities|FlowControl|Switch|SwitchonEnum_LevelElementsTypes (Variables|Default|GetNextWorld)
        (:NewEnumerator1
          (Variables|Default|SetNextWorld "NewEnumerator2")
          (if (not Is%20Instant)
            (bind _opacity (Timeline|Timeline_0 PlayFromStart)
              (:Update
                (Rendering|Material|SetScalarParameterValue "/Game/Materials/SahdeInOut/MPC_Worlds.MPC_Worlds" "Opacity2" _opacity :!class /Script/Engine.KismetMaterialLibrary)
                (Rendering|Material|SetScalarParameterValue "/Game/Materials/SahdeInOut/MPC_Worlds.MPC_Worlds" "Opacity1" (- 1.0 _opacity) :!class /Script/Engine.KismetMaterialLibrary)
                (for _array_element _lightelements
                  (Default|World2 _array_element)
                  (for _array_element_2 _darkelements
                    (Default|World1 _array_element_2))))
              (:Finished
                (Variables|/Game/Blueprint/Blueprints/SideScrollerCharacter.SideScrollerCharacter_C|SetcanChangeWorld (Variables|Default|GetCharacterRef) true)
                (bind _float (Timeline|ChangeBackToLight PlayFromStart)
                  (:Update
                    (Default|ShadetoBlack (Variables|Default|GetCharacterRef) (* _float -1.0)))
                  (:Finished
                    (bind _returnvalue (Utilities|Time|SetTimerbyEvent (delegate Custom|CallGameOver) (Variables|Default|GetMaxTimeInDarkWorld)))))))))
        (:NewEnumerator2
          (Variables|Default|SetNextWorld "NewEnumerator1")
          (if Is%20Instant
            (Rendering|Material|SetScalarParameterValue "/Game/Materials/SahdeInOut/MPC_Worlds.MPC_Worlds" "Opacity2" 0.0 :!class /Script/Engine.KismetMaterialLibrary)
            (Rendering|Material|SetScalarParameterValue "/Game/Materials/SahdeInOut/MPC_Worlds.MPC_Worlds" "Opacity1" 1.0 :!class /Script/Engine.KismetMaterialLibrary)
            (for _array_element_3 _darkelements :!label _label
              (Default|World2 _array_element_3)
              (for _array_element_4 _lightelements
                (Default|World1 _array_element_4)))
            (Variables|/Game/Blueprint/Blueprints/SideScrollerCharacter.SideScrollerCharacter_C|SetcanChangeWorld (Variables|Default|GetCharacterRef) true)
            (else
              (Utilities|FlowControl|Sequence
                (:then_0
                  (bind _opacity_2 (Timeline|Timeline_1 PlayFromStart)
                    (:Update
                      (Rendering|Material|SetScalarParameterValue "/Game/Materials/SahdeInOut/MPC_Worlds.MPC_Worlds" "Opacity2" (- 1.0 _opacity_2) :!class /Script/Engine.KismetMaterialLibrary)
                      (Rendering|Material|SetScalarParameterValue "/Game/Materials/SahdeInOut/MPC_Worlds.MPC_Worlds" "Opacity1" _opacity_2 :!class /Script/Engine.KismetMaterialLibrary)
                      (goto _label))
                    (:Finished
                      (Default|SwitchBacktoLight (Variables|Default|GetCharacterRef))
                      (Utilities|Time|PauseTimerbyHandle _returnvalue))))
                (:then_1
                  (Timeline|ChangeBackToLight Stop))))))))))

(event Custom|GameOver
  ;[0 0 0] GameOver
  (Game|OpenLevel(byName) "LVL_Hub"))

(event Custom|CallGameOver
  (Default|Die (Variables|Default|GetCharacterRef)))

(event Custom|Load
  (Utilities|IsValid (Variables|Default|GetCharacterRef)
    (:Is%20Not%20Valid
      (bind _asside_scroller_character (Utilities|Casting|CastToSideScrollerCharacter (Game|Player|GetPlayerPawn 0)))
      (Variables|Default|SetCharacterRef _asside_scroller_character))))

(event EventBeginPlay
  (Utilities|FlowControl|Delay 0.0)
  (bind _outactors (Actor|GetAllActorsOfClass "/Game/Blueprint/Blueprints/LevelElements/ABP_LevelElement.ABP_LevelElement_C"))
  (for _array_element _outactors
    (switch Utilities|FlowControl|Switch|SwitchonEnum_LevelElementsTypes (Variables|/Game/Blueprint/Blueprints/LevelElements/ABP_LevelElement.ABP_LevelElement_C|GetType _array_element)
      (:NewEnumerator1
        (Utilities|Array|Add (Variables|Default|GetDarkElements) _array_element))
      (:NewEnumerator2
        (Utilities|Array|Add (Variables|Default|GetLightElements) _array_element))))
  (CallFunction|ChangeElementType "NewEnumerator2" true))

(event EventTick
  (params (DeltaSeconds :type Float%20%28single-precision%29))
  (CallFunction|Load))

(fn ConstructionScript)