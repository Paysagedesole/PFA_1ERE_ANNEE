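; Niagara particle actor that wanders the side-scroller's Y/Z plane and flees from the player character.
; A looping Move event picks points in a forward cone, traces for WorldStatic obstacles, and either turns to the hit normal or glides there.
; Overlapping Repulse turns it away and boosts speed, Attraction and Acceleration until a move completes.
; Debug trace drawing and a PrintString remain active.
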(event OnComponentBeginOverlap(Repulse)
  (params (OverlappedComponent :type Primitive%20Component%20Object%20Reference) (OtherActor :type Actor%20Object%20Reference) (OtherComp :type Primitive%20Component%20Object%20Reference) (OtherBodyIndex :type Integer) (bFromSweep :type Boolean) (SweepResult :type Hit%20Result%20Structure%20%28by%20ref%29))
  (bind _asside_scroller_character (Utilities|Casting|CastToSideScrollerCharacter OtherActor))
  (Transformation|SetWorldRotation (Variables|Default|GetDefaultSceneRoot) (Math|Conversions|RotationFromXVector (- (Transformation|GetWorldLocation (Variables|Default|GetDefaultSceneRoot)) (Transformation|GetActorLocation _asside_scroller_character))) false false)
  (CallFunction|ChangeParameters true)
  (CallFunction|Move))

(event Custom|Move
  (bind _defaultsceneroot (Variables|Default|GetDefaultSceneRoot))
  (bind _returnvalue (Transformation|GetWorldRotation _defaultsceneroot))
  (bind _returnvalue_2 (Math|Vector|GetForwardVector _returnvalue))
  (bind _returnvalue_3 (Math|Random|RandomUnitVectorinConeinDegrees _returnvalue_2 15.0))
  (bind _returnvalue_4 (Math|Vector|Normalize _returnvalue_3))
  (bind _output_get (Variables|Default|SetRandom _returnvalue_4))
  (bind (_outhit _returnvalue_5) (Collision|LineTraceForObjects (Transformation|GetWorldLocation (Variables|Default|GetDefaultSceneRoot)) (+ (Transformation|GetActorLocation) (Math|Vector|MakeVector 0.0 (.y (* _output_get 5.5e+02)) (.z (* _output_get 5.5e+02)))) (Utilities|Array|MakeArray "ObjectTypeQuery1") false 0 "Persistent"))
  (if _returnvalue_5
    (Transformation|SetWorldRotation (Variables|Default|GetDefaultSceneRoot) (Math|Conversions|RotationFromXVector (.ImpactNormal (Collision|BreakHitResult _outhit))) false false)
    (CallFunction|Move)
    (else
      (Development|PrintString (Utilities|String|ToString(Vector) _returnvalue_4))
      (Components|MoveComponentTo (Variables|Default|GetDefaultSceneRoot) (+ (Transformation|GetActorLocation) (Math|Vector|MakeVector 0.0 (.y (* _output_get 5.5e+02)) (.z (* _output_get 5.5e+02)))) (Transformation|GetActorRotation) false false (Variables|Default|GetSpeed) false)
      (CallFunction|ChangeParameters false)
      (Utilities|FlowControl|Delay 0.2)
      (CallFunction|Move))))

(event Custom|ChangeParameters
  (params (isFast :type Boolean))
  (bind _niagara (Variables|Default|GetNiagara))
  (bind _niagara_2 (Variables|Default|GetNiagara))
  (bind _attraction (Variables|Default|GetAttraction))
  (bind _acceleration (Variables|Default|GetAcceleration))
  (if isFast
    (Effects|Components|ParticleSystem|SetFloatParameter _niagara_2 "Attraction" (* 2.0 _attraction))
    (Effects|Components|ParticleSystem|SetFloatParameter _niagara_2 "Acceleration" (* 2.0 _acceleration))
    (Variables|Default|SetSpeed 5.0)
    (else
      (Effects|Components|ParticleSystem|SetFloatParameter _niagara "Attraction" _attraction)
      (Effects|Components|ParticleSystem|SetFloatParameter _niagara "Acceleration" _acceleration)
      (Variables|Default|SetSpeed 1e+01))))

(event EventBeginPlay
  (CallFunction|Move))

(event Collision|EventActorBeginOverlap
  (params (OtherActor :type Actor%20Object%20Reference)))

(event EventTick
  (params (DeltaSeconds :type Float%20%28single-precision%29)))

(fn ConstructionScript
  (bind _niagara (Variables|Default|GetNiagara))
  (Effects|Components|ParticleSystem|SetFloatParameter _niagara "Acceleration" (Variables|Default|GetAcceleration))
  (Effects|Components|ParticleSystem|SetFloatParameter _niagara "Attraction" (Variables|Default|GetAttraction)))