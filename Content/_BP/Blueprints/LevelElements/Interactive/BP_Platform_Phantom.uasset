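; Phantom platform level element that exposes Show and Hide events to toggle its timeline-driven behavior.
; On BeginPlay it runs the parent logic, then calls Hide only if the first overlapping SideScrollerCharacter is valid.
; Show starts the timeline and Hide stops it, with no visibility or collision changes in this graph.
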(event EventBeginPlay
  (|CallParentFunction)
  (Utilities|Casting|CastToSideScrollerCharacter (Utilities|Array|Get(acopy) (Collision|GetOverlappingActors "/Game/_BP/Blueprints/SideScrollerCharacter.SideScrollerCharacter_C" :!class /Script/Engine.Actor)))
  (CallFunction|Hide))

(event Collision|EventActorBeginOverlap
  (params (OtherActor :type Actor%20Object%20Reference))
  (|CallParentFunction OtherActor) ; This node is disabled and will not be called.\nDrag off pins to build functionality.
)

(event EventTick
  (params (DeltaSeconds :type Float%20%28single-precision%29)))

(event EventHide
  (CallFunction|StopTimeline))

(event EventShow
  (CallFunction|StartTimeline))

(fn ConstructionScript
  (|CallParentFunction))