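; BP_Door1 is an interactive level door that opens by sliding its mesh upward and can be reset to closed.
; OpenDoor eases the mesh up, hides the door, disables collision, then adds itself to the UsedDoors list on the SideScrollerCharacter found as its owner's owner.
; CloseDoor snaps the mesh back, clears IsUsed on its owning BP_DoorTrigger, and restores visibility and collision.
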(event Custom|OpenDoor
  (Components|MoveComponentTo (Variables|Default|GetStaticMesh) "0, 0,500.000000" "0, 0, 0" true true 3.2 false)
  (Rendering|SetVisibility (Variables|Default|GetScene) false true)
  (Collision|SetActorEnableCollision false)
  (bind _asside_scroller_character (Utilities|Casting|CastToSideScrollerCharacter (Components|GetOwner (Components|GetOwner))))
  (Utilities|Array|AddUnique (Variables|/Game/_BP/Blueprints/SideScrollerCharacter.SideScrollerCharacter_C|GetusedDoors _asside_scroller_character) self))

(event Custom|CloseDoor
  (Transformation|SetRelativeLocation (Variables|Default|GetStaticMesh) "0, 0, 0" false false)
  (bind _asbp_door_trigger (Utilities|Casting|CastToBP_DoorTrigger (Components|GetOwner)))
  (Variables|/Game/_BP/Blueprints/LevelElements/Interactive/BP_DoorTrigger.BP_DoorTrigger_C|SetisUsed _asbp_door_trigger false)
  (Rendering|SetVisibility (Variables|Default|GetScene) true true)
  (Collision|SetActorEnableCollision true))

(event EventBeginPlay)

(event Collision|EventActorBeginOverlap
  (params (OtherActor :type Actor%20Object%20Reference)))

(event EventTick
  (params (DeltaSeconds :type Float%20%28single-precision%29)))

(fn ConstructionScript)