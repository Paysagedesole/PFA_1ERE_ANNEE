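; Invisible platform for a side-scroller that can be revealed, becoming solid to pawns, and later fades out again.
; Show makes it focusable, blocks the Pawn channel, pauses any pending hide timer and plays an opacity timeline on a dynamic material.
; Hide starts a delay timer that reverses the timeline.
; When the reversed timeline reaches its Disappeared event, pawn collision is ignored and focus is turned off.
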(event Custom|HideTimeline
  (bind (_direction _float) (Timeline|Become%20Visible Reverse)
    (:Update
      (Rendering|Material|SetScalarParameterValue (Variables|Default|GetMaterial) "Opacity" _float :!class /Script/Engine.MaterialInstanceDynamic))
    (:Disappeared
      (switch Utilities|FlowControl|Switch|SwitchonETimelineDirection _direction
        (:Backward
          (Collision|SetCollisionResponsetoChannel (Variables|Default|GetStaticMesh) "ECC_Pawn" "ECR_Ignore")
          (Variables|Default|SetisFocusable false))))))

(event EventBeginPlay
  (|CallParentFunction)
  (Components|Timeline|SetPlayRate (Variables|Default|GetBecome%20Visible) (Variables|Invisible|GetInvisibleSwapSpeed))
  (bind _returnvalue (Rendering|Material|CreateDynamicMaterialInstance (Variables|Default|GetStaticMesh) 0 "/Game/Materials/SahdeInOut/MI_InvisiblePlatform.MI_InvisiblePlatform" "None" :!class /Script/Engine.PrimitiveComponent))
  (Variables|Default|SetMaterial _returnvalue)
  (Utilities|FlowControl|Delay 0.0))

(event Collision|EventActorBeginOverlap
  (params (OtherActor :type Actor%20Object%20Reference))
  (|CallParentFunction OtherActor) ; This node is disabled and will not be called.\nDrag off pins to build functionality.
)

(event EventTick
  (params (DeltaSeconds :type Float%20%28single-precision%29)))

(event EventHide
  (bind _returnvalue (Utilities|Time|SetTimerbyEvent (delegate Custom|HideTimeline) (Variables|Invisible|GetDelay))))

(event EventShow
  (Variables|Default|SetisFocusable true)
  (Collision|SetCollisionResponsetoChannel (Variables|Default|GetStaticMesh) "ECC_Pawn" "ECR_Block")
  (Utilities|Time|PauseTimerbyHandle (stale EventHide _returnvalue))
  (bind (_direction _float) (Timeline|Become%20Visible Play)
    (:Update
      (Rendering|Material|SetScalarParameterValue (Variables|Default|GetMaterial) "Opacity" _float :!class /Script/Engine.MaterialInstanceDynamic))
    (:Disappeared
      (switch Utilities|FlowControl|Switch|SwitchonETimelineDirection _direction
        (:Backward
          (Collision|SetCollisionResponsetoChannel (Variables|Default|GetStaticMesh) "ECC_Pawn" "ECR_Ignore")
          (Variables|Default|SetisFocusable false))))))

(fn ConstructionScript
  (|CallParentFunction))