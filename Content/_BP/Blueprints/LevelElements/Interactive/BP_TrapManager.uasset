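; Kill-zone trap strip that calls Die on any SideScrollerCharacter overlapping its box and takes part in world switching.
; The construction script, unless flagged finished, sizes and offsets the box and lays out a centred row of meshes along Y from Size and TrapSize.
; BeginPlay applies a Dark or Light shade-in/out material by Type.
; World1 enables actor collision and World2 disables it, independent of Type.
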(event OnComponentBeginOverlap(Box)
  (params (OverlappedComponent :type Primitive%20Component%20Object%20Reference) (OtherActor :type Actor%20Object%20Reference) (OtherComp :type Primitive%20Component%20Object%20Reference) (OtherBodyIndex :type Integer) (bFromSweep :type Boolean) (SweepResult :type Hit%20Result%20Structure%20%28by%20ref%29))
  (bind _asside_scroller_character (Utilities|Casting|CastToSideScrollerCharacter OtherActor))
  (Default|Die _asside_scroller_character))

(event EventBeginPlay
  (|CallParentFunction)
  (for _array_element (Variables|Default|GetMeshs)
    (switch Utilities|FlowControl|Switch|SwitchonEnum_LevelElementsTypes (Variables|Default|GetType)
      (:NewEnumerator1
        (Rendering|Material|SetMaterial _array_element 0 "/Game/Materials/SahdeInOut/MI_ShadeInOut_Inst1.MI_ShadeInOut_Inst1"))
      (:NewEnumerator2
        (Rendering|Material|SetMaterial (Variables|Default|GetStaticMesh) 0 "/Game/Materials/SahdeInOut/MI_ShadeInOut_Inst2.MI_ShadeInOut_Inst2")))))

(event Collision|EventActorBeginOverlap
  (params (OtherActor :type Actor%20Object%20Reference)))

(event EventTick
  (params (DeltaSeconds :type Float%20%28single-precision%29)))

(event EventWorld1
  (Collision|SetActorEnableCollision true))

(event EventWorld2
  (Collision|SetActorEnableCollision false))

(fn ConstructionScript
  (bind _trapsize (Variables|Default|GettrapSize))
  (bind _size (Variables|Default|GetSize))
  (bind _returnvalue (/ _size _trapsize))
  (bind _returnvalue_2 (Math|Float|Truncate _returnvalue))
  (if (not (Variables|Default|GetFINNISHED))
    (Components|Box|SetBoxExtent (Variables|Default|GetBox) (Math|Vector|MakeVector 64.0 (* (Variables|Default|GetSize) (- 1.0 (Variables|Default|GetadjustColliderSize))) 64.0) true)
    (Transformation|SetRelativeLocation (Variables|Default|GetBox) (Math|Vector|MakeVector 0.0 (Variables|Default|GetOffset) 0.0) false false)
    (|CallParentFunction)
    (for _index (range 0 _returnvalue_2)
      (bind _returnvalue_3 (AddComponent|AddStaticMeshComponent false (Math|Transform|MakeTransform (Math|Vector|MakeVector 0.0 (* (- _index (/ _returnvalue_2 2)) (Variables|Default|GettrapSize)) 0.0) "0, 0, 0" "1,1,1")))
      (Utilities|Array|AddUnique (Variables|Default|GetMeshs) _returnvalue_3))))